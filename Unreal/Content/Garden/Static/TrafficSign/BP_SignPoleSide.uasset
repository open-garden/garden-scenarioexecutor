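; BP_SignPoleSide is a construction-time tool that lines a spline with instanced copies of one static mesh, apparently for traffic sign pole sides.
; Each pair of neighbouring spline points forms a straight segment, filled with whole meshes sized from their X bounds and ScaleOffset.
; Instances stretch along X to fit the segment exactly and face the next point, with an option to keep them vertically aligned using yaw only.
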(event EventBeginPlay)

(event Collision|EventActorBeginOverlap
  (params (OtherActor :type Actor%20Object%20Reference)))

(event EventTick
  (params (DeltaSeconds :type Float%20%28single-precision%29)))

(fn ConstructionScript
  (bind _returnvalue (AddComponent|AddInstancedStaticMeshComponent false))
  (Components|StaticMesh|SetStaticMesh _returnvalue (Variables|Default|GetstaticMesh))
  (Variables|Default|SetMeshLenght (* (- (.x (.Max (Components|StaticMesh|GetLocalBounds _returnvalue))) (.x (.Min (Components|StaticMesh|GetLocalBounds _returnvalue)))) (Variables|Default|GetScaleOffset)))
  (for _index (range 0 (- (Spline|GetNumberOfSplinePoints (Variables|Default|GetSpline)) 2))
    (CallFunction|SpawnBetween2Points _index _returnvalue (Variables|Default|GetSpline))))

(fn SpawnBetween2Points
  (params (PointIndex :type Integer) (InstancedStaticMesh :type Instanced%20Static%20Mesh%20Component%20Object%20Reference) (Spline :type Spline%20Component%20Object%20Reference))
  (bind _location (Spline|GetLocationandTangentatSplinePoint Spline PointIndex "Local"))
  (bind _returnvalue (+ PointIndex 1))
  (bind _meshlenght (Variables|Default|GetMeshLenght))
  (bind _location_2 (Spline|GetLocationandTangentatSplinePoint Spline _returnvalue "Local"))
  (bind _returnvalue_2 (Math|Rotator|FindLookatRotation _location _location_2))
  (bind (_scale _number_of_meshes) (CallFunction|CalculateNumberOfMeshes _meshlenght (Math|Vector|VectorLength (- _location_2 _location))))
  (for _index (range 0 _number_of_meshes)
    ;[1 1 1] Switch between Z alignment
    (if (Variables|Default|Getverticaly%20Aligned)
      (Variables|Default|SetFinalTransform (Math|Rotator|MakeRotator 0.0 0.0 (.Yaw (Math|Rotator|BreakRotator _returnvalue_2))))
      (else
        (Variables|Default|SetFinalTransform _returnvalue_2)))
    (Components|InstancedStaticMesh|AddInstance InstancedStaticMesh (Math|Transform|MakeTransform (+ (* (* (Math|Rotator|GetRotationXVector _returnvalue_2) _index) (* _scale _meshlenght)) _location) (Variables|Default|GetFinalTransform) (Math|Vector|MakeVector _scale 1.0 1.0)))))

(fn CalculateNumberOfMeshes
  (params (MeshLenght :type Float%20%28single-precision%29) (TotalDistance :type Float%20%28single-precision%29))
  (bind _returnvalue (/ TotalDistance MeshLenght))
  (bind _returnvalue_2 (Math|Float|Truncate _returnvalue))
  (bind _returnvalue_3 (* _returnvalue_2 MeshLenght))
  ;[1 1 1] Remember kids. NEVER, By any chance, allow your calculations to accidentaly divide by 0.
  (if (not (or (== _returnvalue_3 0.0) (== TotalDistance 0.0)))
    (return (/ TotalDistance _returnvalue_3) (- _returnvalue_2 1))))