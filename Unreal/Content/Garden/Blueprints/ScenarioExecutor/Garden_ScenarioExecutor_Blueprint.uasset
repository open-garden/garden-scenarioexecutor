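; Scenario executor bridge that mirrors an external scenario's vehicles in the Garden level.
; Tick retries the connection, then reads integer parameters scaled to transforms, spawning vehicles by model ID or destroying all when the scenario flag is zero.
; Spawned vehicles get a GardenVehicle component, vehicle and biker anim classes, and stopped attached audio.
; The audio listener follows the ego car; an uncalled debug function prints collision bounds per vehicle class.
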(event EventBeginPlay
  (Class|GardenBlueprintFunctionLibrary|InitializeScenarioExecutor))

(event EventTick
  (params (DeltaSeconds :type Float%20%28single-precision%29))
  (bind _returnvalue (Class|GardenBlueprintFunctionLibrary|IsConnected))
  (if _returnvalue
    (CallFunction|SpawnVehicle)
    (CallFunction|SetAudioListener)
    (else
      (Class|GardenBlueprintFunctionLibrary|ConnectScenarioExecutor))))

(event EventEndPlay
  (params (EndPlayReason :type EEndPlayReason%20Enum :default "Destroyed"))
  (Class|GardenBlueprintFunctionLibrary|DisconnectScenarioExecutor))

(fn ConstructionScript)

(fn SpawnVehicle
  (bind _gardenvehicleblueprintarray (Variables|Default|GetGardenVehicleBlueprintArray))
  (bind _returnvalue (Class|GardenBlueprintFunctionLibrary|GetScenarioExeInfoParam))
  (if (!= _returnvalue 0)
    (bind _returnvalue_2 (Class|GardenBlueprintFunctionLibrary|GetNewVehicleID))
    (bind _returnvalue_3 (Class|GardenBlueprintFunctionLibrary|GetParamLen))
    (bind _returnvalue_4 (Class|GardenBlueprintFunctionLibrary|GetOtherCarInfoParam (* _returnvalue_3 _returnvalue_2)))
    (if (!= _returnvalue_4 0)
      (bind _returnvalue_5 (Class|GardenBlueprintFunctionLibrary|GetModelId (+ (* _returnvalue_3 _returnvalue_2) 1)))
      (bind _returnvalue_6 (Class|GardenBlueprintFunctionLibrary|GetOtherCarInfoParam (+ (* _returnvalue_3 _returnvalue_2) 21)))
      (bind _returnvalue_7 (Class|GardenBlueprintFunctionLibrary|GetOtherCarInfoParam (+ (+ (* _returnvalue_3 _returnvalue_2) 21) 1)))
      (bind _returnvalue_8 (Class|GardenBlueprintFunctionLibrary|GetOtherCarInfoParam (+ (+ (+ (* _returnvalue_3 _returnvalue_2) 21) 1) 1)))
      (bind _returnvalue_9 (Class|GardenBlueprintFunctionLibrary|GetOtherCarInfoParam (+ (+ (+ (+ (* _returnvalue_3 _returnvalue_2) 21) 1) 1) 1)))
      (bind _returnvalue_10 (Class|GardenBlueprintFunctionLibrary|GetOtherCarInfoParam (+ (+ (+ (+ (+ (* _returnvalue_3 _returnvalue_2) 21) 1) 1) 1) 1)))
      (bind _returnvalue_11 (Class|GardenBlueprintFunctionLibrary|GetOtherCarInfoParam (+ (+ (+ (+ (+ (+ (* _returnvalue_3 _returnvalue_2) 21) 1) 1) 1) 1) 1)))
      (bind (_vehicleclass _animclass _soundcue) (CallFunction|GetSpawnVehicleClass _returnvalue_5))
      (bind _returnvalue_12 (Game|SpawnActorfromClass _vehicleclass (Math|Transform|MakeTransform (Math|Vector|MakeVector (/ (Math|Conversions|ToFloat(Integer) _returnvalue_6) 1e+02) (/ (Math|Conversions|ToFloat(Integer) _returnvalue_7) 1e+02) (/ (Math|Conversions|ToFloat(Integer) _returnvalue_8) 1e+02)) (Math|Rotator|MakeRotator (/ (Math|Conversions|ToFloat(Integer) _returnvalue_9) 1e+04) (/ (Math|Conversions|ToFloat(Integer) _returnvalue_10) 1e+04) (/ (Math|Conversions|ToFloat(Integer) _returnvalue_11) 1e+04))) "AlwaysSpawn" 0 0 0))
      (CallFunction|SetActor _returnvalue_12 _animclass _soundcue)
      (Utilities|Array|Add (Variables|Default|GetGardenVehicleBlueprintArray) _returnvalue_12))
    (else
      (for _array_element _gardenvehicleblueprintarray
        (Actor|DestroyActor _array_element))
      (Utilities|Array|Clear _gardenvehicleblueprintarray)
      (Class|GardenBlueprintFunctionLibrary|SetNewVehicleID))))

(fn GetSpawnVehicleClass
  (params (ModelId :type String))
  (for _array_element (Variables|Default|GetGardenVehicleClassArray)
    (if (Utilities|Enum|Equal(Enum) ModelId (.ModelID (Utilities|Struct|BreakGarden_VehicleClass_Structure _array_element)))
      (return (.VehicleClass (Utilities|Struct|BreakGarden_VehicleClass_Structure _array_element)) (.VehicleAnimClass (Utilities|Struct|BreakGarden_VehicleClass_Structure _array_element)) (.SoundCue (Utilities|Struct|BreakGarden_VehicleClass_Structure _array_element))))))

(fn SetActor
  (params (Actor :type Base%20Vehicle%20Pawn%20Object%20Reference) (AnimClass :type Anim%20Instance%20Class%20Reference) (SoundCue :type Sound%20Cue%20Object%20Reference))
  (Utilities|FlowControl|Sequence
    (:then_0
      (bind _returnvalue (AddComponent|AddGardenVehicleComponent Actor))
      (bind _output_get (LocalVariables|SetGardenVehicleComponent _returnvalue))
      (bind _output_get_2 (Variables|/Game/Garden/Blueprints/ScenarioExecutor/Vehicles/Garden_Vehicle_Component.Garden_Vehicle_Component_C|SetActor _output_get Actor))
      (LocalVariables|SetMesh (Variables|/Script/PhysXVehicles.WheeledVehicle|GetMesh _output_get_2)))
    (:then_1
      (Class|SkeletalMeshComponent|SetAnimClass (LocalVariables|GetMesh) AnimClass)
      (bind _asskeletal_mesh_component (Utilities|Casting|CastToSkeletalMeshComponent (Components|GetChildComponent (LocalVariables|GetMesh) 3)))
      (Class|SkeletalMeshComponent|SetAnimClass _asskeletal_mesh_component "/Game/Garden/Blueprints/ScenarioExecutor/Vehicles/2WheeledVehicle/Garden_Biker_AnimBlueprint.Garden_Biker_AnimBlueprint_C"))
    (:then_2
      (if (!= SoundCue 0)
        (bind _returnvalue_2 (Audio|SpawnSoundAttached SoundCue (LocalVariables|GetMesh) "Vehicle_Base" "0, 0,2.000000" "0, 0, 0" "KeepRelativeOffset" true 1.0 1.0 0.0 0 0 false))
        (Audio|Components|Audio|Stop _returnvalue_2)
        (Variables|/Game/Garden/Blueprints/ScenarioExecutor/Vehicles/Garden_Vehicle_Component.Garden_Vehicle_Component_C|SetAudio (LocalVariables|GetGardenVehicleComponent) _returnvalue_2)))))

(fn SetAudioListener
  (bind _returnvalue (Class|KismetSystemLibrary|MakeLiteralInteger))
  (bind _returnvalue_2 (+ _returnvalue 1))
  (bind _returnvalue_3 (+ _returnvalue_2 1))
  (bind _returnvalue_4 (+ _returnvalue_3 1))
  (bind _returnvalue_5 (+ _returnvalue_4 1))
  (bind _returnvalue_6 (Class|GardenBlueprintFunctionLibrary|GetEgoCarInfoParam _returnvalue))
  (bind _returnvalue_7 (Class|GardenBlueprintFunctionLibrary|GetEgoCarInfoParam _returnvalue_2))
  (bind _returnvalue_8 (Class|GardenBlueprintFunctionLibrary|GetEgoCarInfoParam _returnvalue_3))
  (bind _returnvalue_9 (Class|GardenBlueprintFunctionLibrary|GetEgoCarInfoParam _returnvalue_4))
  (bind _returnvalue_10 (Class|GardenBlueprintFunctionLibrary|GetEgoCarInfoParam _returnvalue_5))
  (bind _returnvalue_11 (Class|GardenBlueprintFunctionLibrary|GetEgoCarInfoParam (+ _returnvalue_5 1)))
  (Class|PlayerController|SetAudioListenerOverride (Game|GetPlayerController 0) 0 (Math|Vector|MakeVector (/ (Math|Conversions|ToFloat(Integer) _returnvalue_6) 1e+02) (/ (Math|Conversions|ToFloat(Integer) _returnvalue_7) 1e+02) (/ (Math|Conversions|ToFloat(Integer) _returnvalue_8) 1e+02)) (Math|Rotator|MakeRotator (/ (Math|Conversions|ToFloat(Integer) _returnvalue_9) 1e+04) (/ (Math|Conversions|ToFloat(Integer) _returnvalue_10) 1e+04) (/ (Math|Conversions|ToFloat(Integer) _returnvalue_11) 1e+04))))

(fn DebugPrintBounds
  (for (_array_element _array_index) (Variables|Default|GetGardenVehicleClassArray)
    (bind _returnvalue (Game|SpawnActorfromClass (.VehicleClass (Utilities|Struct|BreakGarden_VehicleClass_Structure _array_element)) (Math|Transform|MakeTransform (Math|Vector|MakeVector (* _array_index 6e+02) 0.0 2e+02)) "AlwaysSpawn" 0 0 0))
    (Development|PrintString (.ModelID (Utilities|Struct|BreakGarden_VehicleClass_Structure _array_element)))
    (for _array_element_2 (Actor|GetComponentsByClass _returnvalue "/Script/Engine.StaticMeshComponent")
      (if (Utilities|Enum|Equal(Enum) (Utilities|GetObjectName _array_element_2) "CustomCollision")
        (Development|PrintString (Utilities|String|ToString(Vector) (* (.BoxExtent (Collision|GetComponentBounds _array_element_2)) "2.000000,2.000000,2.000000")) true true "(R=0.000000,G=0.660000,B=1.000000,A=1.000000)" 6e+01)))))